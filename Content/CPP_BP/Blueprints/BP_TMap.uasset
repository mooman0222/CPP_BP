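; BP_TMap is a Blueprint that exercises map operations on FruitMap, an integer-keyed map of fruit names.
; On BeginPlay, a Sequence adds an entry, removes another by key, then gathers the remaining keys.
; It loops over those keys, looks up each value with Find and prints the key and value pair as a string.
; The construction script is empty.
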(event `self.ReceiveBeginPlay`
  (bind _fruitmap (`self.FruitMap`))
  (`|ExecutionSequence`
    (:`then_0`
      (`BlueprintMapLibrary.Map_Add` (`self.FruitMap`) 12 "Orange"))
    (:`then_1`
      (`BlueprintMapLibrary.Map_Remove` (`self.FruitMap`) 3))
    (:`then_2`
      (bind _keys (`BlueprintMapLibrary.Map_Keys` _fruitmap))
      (for _array_element _keys
        (`KismetSystemLibrary.PrintString` (`KismetStringLibrary.Concat_StrStr` "Key : " (`KismetStringLibrary.Conv_IntToString` _array_element) " Values : " (`BlueprintMapLibrary.Map_Find` _fruitmap _array_element)))))))

(fn `UserConstructionScript`)