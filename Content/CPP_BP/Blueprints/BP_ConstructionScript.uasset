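; BP_ConstructionScript is an actor that demonstrates configuring a PointLight component through its Construction Script.
; The Construction Script applies the visibility, intensity and light color variables to the light, so edits to those properties show on the placed actor.
; At BeginPlay it prints a message string with a configurable text color and duration.
; The overlap and Tick events are unused stubs.
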(event `self.ReceiveBeginPlay`
  ;[1 1 1] Hello Worldと出力する
  (`KismetSystemLibrary.PrintString` (`self.Message`) true true (`self.TextColor`) (`self.Duration`)) ; Hello World!と出力する
)

(fn `UserConstructionScript`
  ;[1 1 1] PointLightの表示/非表示
  (`SceneComponent.SetVisibility` (`self.PointLight`) (`self.IsVisible`) false)
  ;[1 1 1] PointLightのIntensityを設定する
  (`LightComponent.SetIntensity` (`self.PointLight`) (`self.Intensity`))
  ;[1 1 1] PointLightのLightColorを変更する
  (`LightComponent.SetLightColor` (`self.PointLight`) (`self.LightColor`) true))