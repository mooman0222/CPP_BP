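; BP_Calculation is a practice actor that prints arithmetic results to the screen and carries a configurable point light.
; On BeginPlay it prints a message, then the result of a Math Expression node fed by CalcVarA and CalcVarB.
; The Construction Script applies visibility, intensity and color variables to the PointLight.
; Separate add, subtract, multiply and divide print nodes remain in the event graph but never run.
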(event EventBeginPlay
  ;[1 1 1] Hello Worldと出力する
  (Development|PrintString (Variables|PrintString|GetMessage) true true (Variables|PrintString|GetTextColor) (Variables|PrintString|GetDuration)) ; Hello World!と出力する
  ;[1 1 1] Math Expression
  (Development|PrintString (Utilities|String|ToString(Float) (|(A+B) (Math|Conversions|ToFloat(Integer) (Variables|Calculation|GetCalcVarA)) (Math|Conversions|ToFloat(Integer) (Variables|Calculation|GetCalcVarB)))) true true "(R=0.950000,G=0.000000,B=0.000000,A=1.000000)"))

(event Collision|EventActorBeginOverlap
  (params (OtherActor :type Actor%20Object%20Reference)))

(event EventTick
  (params (DeltaSeconds :type Float%20%28single-precision%29)))

(fn ConstructionScript
  ;[1 1 1] PointLightの表示/非表示
  (Rendering|SetVisibility (Variables|Default|GetPointLight) (Variables|PointLight|GetIsVisible) false)
  ;[1 1 1] PointLightのIntensityを設定する
  (Rendering|Components|Light|SetIntensity (Variables|Default|GetPointLight) (Variables|PointLight|GetIntensity))
  ;[1 1 1] PointLightのLightColorを変更する
  (Rendering|Components|Light|SetLightColor (Variables|Default|GetPointLight) (Variables|PointLight|GetLightColor) true))