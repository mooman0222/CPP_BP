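; BP_Function is a practice actor with a point light that demonstrates variables, branching, enums and functions by printing to screen.
; On BeginPlay it prints either a configurable message or the result of PrintCalcResult, which switches on CalcType to add (via the Sum function), subtract, multiply or divide two variables.
; The construction script applies the light's visibility, intensity and color from variables.
; Leftover branch, switch and math-expression experiments in the event graph never run.
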(event `self.ReceiveBeginPlay`
  (if (`self.IsPrintHello`)
    ;[1 1 1] Hello Worldと出力する
    (`KismetSystemLibrary.PrintString` (`self.Message`) true true (`self.TextColor`) (`self.Duration`)) ; Hello World!と出力する
    (else
      (`self.PrintCalcResult`))))

(fn `PrintCalcResult`
  (bind _calcvara (`self.CalcVarA`))
  (bind _calcvarb (`self.CalcVarB`))
  (bind _duration (`self.Duration`))
  (switch `/Game/CPP_BP/Blueprints/EBPCalcType` (`self.CalcType`)
    (:`NewEnumerator0`
      ;[0.77 0 0] 足し算
      (`KismetSystemLibrary.PrintString` (`KismetStringLibrary.Conv_IntToString` (`self.Sum` _calcvara _calcvarb)) true true (struct :`R` 0.83 :`A` 1.0) _duration))
    (:`NewEnumerator1`
      ;[1 0.9906 0.3] 引き算
      (`KismetSystemLibrary.PrintString` (`KismetStringLibrary.Conv_IntToString` (- _calcvara _calcvarb)) true true (struct :`R` 1.0 :`G` 0.952215 :`B` 0.11 :`A` 1.0) _duration))
    (:`NewEnumerator2`
      ;[0 0.94 0.03154] 乗算
      (`KismetSystemLibrary.PrintString` (`KismetStringLibrary.Conv_IntToString` (* _calcvara _calcvarb)) true true (struct :`G` 0.95 :`B` 0.012752 :`A` 1.0) _duration))
    (:`NewEnumerator3`
      ;[1 0.19 0.875] 割り算
      (`KismetSystemLibrary.PrintString` (`KismetStringLibrary.Conv_DoubleToString` (/ _calcvara _calcvarb)) true true (struct :`R` 1.0 :`G` 0.27 :`B` 0.990201 :`A` 1.0) _duration))))

(fn `Sum`
  (params (A :type "Integer (by ref)") (B :type "Integer (by ref)"))
  (returns (ReturnValue :type Integer))
  (locals (LocalResult :type Integer))
  (bind _output_get (set `local.LocalResult` (+ A B)))
  (return _output_get))

(fn `UserConstructionScript`
  ;[1 1 1] PointLightの表示/非表示
  (`SceneComponent.SetVisibility` (`self.PointLight`) (`self.IsVisible`) false)
  ;[1 1 1] PointLightのIntensityを設定する
  (`LightComponent.SetIntensity` (`self.PointLight`) (`self.Intensity`))
  ;[1 1 1] PointLightのLightColorを変更する
  (`LightComponent.SetLightColor` (`self.PointLight`) (`self.LightColor`) true))