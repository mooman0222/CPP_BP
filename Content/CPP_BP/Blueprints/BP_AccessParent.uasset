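; BP_AccessParent is a parent Blueprint that appears to demonstrate public, protected and private access, judging by its names.
; Three functions each print the object's display name, an access-level label and the matching VarPublicNum, VarProtectedNum or VarPrivateNum value.
; The event graph calls all three functions only from nodes that never run, and its events and construction script are empty.
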(event `self.ReceiveBeginPlay`)

(fn `CallPrivateFunc`
  (`KismetSystemLibrary.PrintString` (`KismetStringLibrary.Concat_StrStr` (`KismetSystemLibrary.GetDisplayName` self) ":Call Private Func" (`KismetStringLibrary.Conv_IntToString` (`self.VarPrivateNum`)))))

(fn `CallProtectedFunc`
  (`KismetSystemLibrary.PrintString` (`KismetStringLibrary.Concat_StrStr` (`KismetSystemLibrary.GetDisplayName` self) ":Call Pritected Func" (`KismetStringLibrary.Conv_IntToString` (`self.VarProtectedNum`)))))

(fn `CallPublicFunc`
  (`KismetSystemLibrary.PrintString` (`KismetStringLibrary.Concat_StrStr` (`KismetSystemLibrary.GetDisplayName` self) ":Call PublicFunc" (`KismetStringLibrary.Conv_IntToString` (`self.VarPublicNum`)))))

(fn `UserConstructionScript`)